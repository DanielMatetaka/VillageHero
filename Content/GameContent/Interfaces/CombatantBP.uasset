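; Combatant character Blueprint handling health, death, faction, a holstered or hand-held weapon, and melee combos.
; On BeginPlay it spawns its weapon and attaches it to the holster socket; equip toggling moves it between holster and right hand.
; Attack steps through the weapon's montage moveset, queuing follow-ups that animation-notification events play or reset.
; Hit detection sphere-traces forward from the hand by weapon range, sending weapon damage through the Combatant interface.
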(event EventBeginPlay
  (if (Utilities|IsValidClass (Variables|Equipment|GetWeapon))
    (bind _returnvalue (Game|SpawnActorfromClass (Variables|Equipment|GetWeapon) (Transformation|GetActorTransform) "Undefined" 0 0))
    (CallFunction|SetPrimaryWeapon _returnvalue)))

(event EventSustainDamage
  (params (Damage :type Float%20%28single-precision%29))
  (bind _output_get (Variables|Combat|SetHealth (- (Variables|Combat|GetHealth) Damage)))
  (if (<= _output_get 0.0)
    (CallFunction|OnDeath)))

(event EventAddHealth
  (params (Health :type Float%20%28single-precision%29))
  (Variables|Combat|SetHealth (+ (Variables|Combat|GetHealth) Health)))

(event EventSetPrimaryWeapon
  (params (Weapon :type Weapon%20BP%20Object%20Reference))
  (Variables|Equipment|SetPrimaryWeapon Weapon)
  (CallFunction|HolsterWeapon)
  (Development|PrintString "Hello"))

(event EventOnDeath
  (bind _isdead (CallFunction|IsDead))
  (if (not _isdead)
    (Variables|Combat|SetIsDead? true)
    (Components|DestroyComponent (Variables|Collision|GetCapsuleComponent))))

(event EventAttack
  (bind _isequipped (CallFunction|IsEquipped))
  (if _isequipped
    (if (Variables|Attack|GetIsAttacking?)
      (CallFunction|SetCanCombo true)
      (else
        (Variables|Attack|SetIsAttacking? true)
        (Utilities|PlayComboAnimation)))))

(event EventSetCanCombo
  (params (CanCombo :type Boolean))
  (Variables|Attack|SetCanCombo? CanCombo))

(event EventHolsterWeapon
  (CallFunction|AttachtoSocket "WeaponHolster")
  (Variables|Equipment|SetIsEquipped? false))

(event EventUnholsterWeapon
  (CallFunction|AttachtoSocket "RightHandWeapon")
  (Variables|Equipment|SetIsEquipped? true))

(event EventToggleEquip
  (bind _isequipped (CallFunction|IsEquipped))
  (bind _output_get (Variables|Equipment|SetIsEquipped? (not _isequipped)))
  (if _output_get
    (CallFunction|UnholsterWeapon)
    (else
      (CallFunction|HolsterWeapon))))

(event EventOnComboAttack
  (bind _cancombo (CallFunction|CanCombo))
  (if _cancombo
    (CallFunction|SetCanCombo false)
    (Utilities|PlayComboAnimation)))

(event EventOnComboReset
  (Variables|Attack|SetCombo 0)
  (Variables|Attack|SetIsAttacking? false)
  (CallFunction|SetCanCombo false))

(event EventPerformMeleeHitDetection
  (bind _mesh (Variables|Character|GetMesh))
  (bind _returnvalue (Transformation|GetSocketLocation _mesh "RightHandWeapon"))
  (bind _range (Class|Weapon|GetRange(Message) (Variables|Equipment|GetPrimaryWeapon)))
  (bind _outhit (Collision|SphereTraceForObjects _returnvalue (+ (* (Math|Vector|GetForwardVector (Transformation|GetActorRotation)) _range) _returnvalue) 5e+01 (Utilities|Array|MakeArray "ObjectTypeQuery3" "ObjectTypeQuery1" "ObjectTypeQuery2") true 0 "ForDuration"))
  ;[1 1 1] Damage the combatant after hit detection
  (if (Utilities|DoesObjectImplementInterface (.hitactor _outhit) "/Game/GameContent/Interfaces/Combatant.Combatant_C")
    (bind _damage (Class|Weapon|GetDamage(Message) (Variables|Equipment|GetPrimaryWeapon)))
    (Class|Combatant|SustainDamage(Message) (.hitactor _outhit) _damage)))

(event EventOnEquip
  (bind _weapon (CallFunction|GetPrimaryWeapon))
  (Utilities|IsValid _weapon
    (:Is%20Valid
      (Animation|PlayAnimMontage "/Game/GameContent/Animations/Equip-Sword-M.Equip-Sword-M" 1.0 "None"))))

(event EventOnUnequip
  (bind _weapon (CallFunction|GetPrimaryWeapon))
  (Utilities|IsValid _weapon
    (:Is%20Valid
      (Animation|PlayAnimMontage "/Game/GameContent/Animations/Equip-Sword-M.Equip-Sword-M" 1.0 "None")
      (CallFunction|OnComboReset))))

(fn ConstructionScript)

(fn AttachtoSocket
  (params (Socket :type Name))
  (bind _weapon (CallFunction|GetPrimaryWeapon))
  (Transformation|SetActorTransform _weapon (Transformation|GetSocketTransform (Variables|Character|GetMesh) Socket "RTS_World"))
  (Transformation|AttachComponentToComponent (Variables|Equipment|GetPrimaryWeapon) (Variables|Character|GetMesh) Socket "KeepWorld" "KeepWorld" "KeepWorld" true))

(fn BelongstoFaction
  (params (Faction :type Faction%20Enum :default "NewEnumerator0"))
  (return (Utilities|Enum|Equal(Enum) Faction (Variables|Faction|GetFaction))))

(fn CanCombo
  (return (Variables|Attack|GetCanCombo?)))

(fn GetFaction
  (return (Variables|Faction|GetFaction)))

(fn GetHealth
  (return (Variables|Combat|GetHealth)))

(fn GetPrimaryWeapon
  (return (Variables|Equipment|GetPrimaryWeapon)))

(fn IsDead
  (return (Variables|Combat|GetIsDead?)))

(fn IsEquipped
  (return (Variables|Equipment|GetIsEquipped?)))