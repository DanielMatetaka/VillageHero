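; PickupBP is a pickup actor that the TopDownCharacter can detect when it enters the pickup area.
; On overlap it registers itself as the character's PickupItem and shows a PickupWidget, created on first use and reused afterwards.
; When the overlap ends it clears that reference and removes the widget from the screen.
; The pickup action itself is not handled in this Blueprint.
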(event OnComponentBeginOverlap(PickupArea)
  (params (OverlappedComponent :type Primitive%20Component%20Object%20Reference) (OtherActor :type Actor%20Object%20Reference) (OtherComp :type Primitive%20Component%20Object%20Reference) (OtherBodyIndex :type Integer) (bFromSweep :type Boolean) (SweepResult :type Hit%20Result%20Structure%20%28by%20ref%29))
  (bind _astop_down_character (Utilities|Casting|CastToTopDownCharacter OtherActor))
  (Variables|/Game/TopDownBP/Blueprints/TopDownCharacter.TopDownCharacter_C|SetPickupItem _astop_down_character self)
  (Utilities|IsValid (Variables|Widget|GetPickupWidget)
    (:Is%20Valid
      (UserInterface|Viewport|AddtoViewport (Variables|Widget|GetPickupWidget) 0))
    (:Is%20Not%20Valid
      (bind _returnvalue (UserInterface|CreateWidget "/Game/GameContent/Interfaces/PickupWidget.PickupWidget_C"))
      (bind _output_get (Variables|Widget|SetPickupWidget _returnvalue))
      (UserInterface|Viewport|AddtoViewport _output_get 0))))

(event OnComponentEndOverlap(PickupArea)
  (params (OverlappedComponent :type Primitive%20Component%20Object%20Reference) (OtherActor :type Actor%20Object%20Reference) (OtherComp :type Primitive%20Component%20Object%20Reference) (OtherBodyIndex :type Integer))
  (bind _astop_down_character (Utilities|Casting|CastToTopDownCharacter OtherActor))
  (Variables|/Game/TopDownBP/Blueprints/TopDownCharacter.TopDownCharacter_C|SetPickupItem _astop_down_character 0)
  (Widget|RemovefromParent (Variables|Widget|GetPickupWidget)))

(fn ConstructionScript)